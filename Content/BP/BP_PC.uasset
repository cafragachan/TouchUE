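; BP_PC is a player controller, apparently a test setup, for viewing a runtime-loaded glTF model with Pixel Streaming input.
; On BeginPlay it downloads a chair GLB via glTFRuntime, spawns it with collision, swaps a material variant and binds click printing.
; Pixel Streamer JSON events containing Category and Item fields pass Item as a float to BP_Pawn's ZoomInput.
; Left click prints the actor under the cursor; alternative load and touch-trace nodes are disconnected.
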(event Custom|LoadAsset
  (params (Asset :type Gl%20TF%20Runtime%20Asset%20Object%20Reference))
  (bind _returnvalue (Game|SpawnActorfromClass :Class "/Script/glTFRuntime.glTFRuntimeAssetActor" :SpawnTransform (Math|Transform|MakeTransform "0, 0, 0") :CollisionHandlingOverride "Undefined" :Asset Asset :StaticMeshConfig (Utilities|Struct|MakeglTFRuntimeStaticMeshConfig "ReadWrite" false true 0 0 "CTF_UseSimpleAndComplex" false "Asset" 0 "(CacheMode=ReadWrite,UberMaterialsOverrideMap=(),MaterialsOverrideMap=(),MaterialsOverrideByNameMap=(),TexturesOverrideMap=(),ImagesOverrideMap=(),bDisableVertexColors=False,bGeneratesMipMaps=False,bMergeSectionsByMaterial=False,SpecularFactor=0.000000,bMaterialsOverrideMapInjectParams=False,ParamsMultiplier=())" 0 "" 0 "IfMissing" "IfMissing" false) :Instigator 0))
  (Rendering|Material|SetMaterial (Actor|GetComponentbyClass _returnvalue "/Script/Engine.StaticMeshComponent") 1 (Utilities|Array|Get(acopy) (Variables|/Script/glTFRuntime.glTFRuntimeAssetActor|GetMaterialVariants _returnvalue) 1))
  (Development|PrintString (Utilities|GetDisplayName (Actor|GetComponentbyClass _returnvalue "/Script/Engine.StaticMeshComponent")))
  (EventDispatchers|BindEventtoOnClicked (Actor|GetComponentbyClass _returnvalue "/Script/Engine.StaticMeshComponent") (delegate Custom|CustomEvent_0)))

(event Custom|CustomEvent_1
  (params (Descriptor :type String))
  (bind _output_get (Variables|Default|SetDescriptor Descriptor))
  (Development|PrintString _output_get true true "(R=1.000000,G=0.000000,B=0.640621,A=1.000000)" 1e+01)
  (if (.Success (Class|PixelStreamerInputComponent|GetJsonStringValue (Variables|Default|GetPSComp) (Variables|Default|GetDescriptor) "Category"))
    (if (.Success (Class|PixelStreamerInputComponent|GetJsonStringValue (Variables|Default|GetPSComp) (Variables|Default|GetDescriptor) "Item"))
      (bind _asbp_pawn (Utilities|Casting|CastToBP_Pawn (Game|Player|GetPlayerPawn 0)))
      (Default|ZoomInput _asbp_pawn (Math|Conversions|ToFloat(Integer) (.StringValue (Class|PixelStreamerInputComponent|GetJsonStringValue (Variables|Default|GetPSComp) (Variables|Default|GetDescriptor) "Item")))))))

(event Custom|CustomEvent_0
  (params (TouchedComponent :type Primitive%20Component%20Object%20Reference) (ButtonPressed :type Key%20Structure :default "None"))
  (Development|PrintString (Utilities|GetDisplayName TouchedComponent)))

(event EventTick
  (params (DeltaSeconds :type Float%20%28single-precision%29)))

(event EventBeginPlay
  (Class|GlTFRuntimeFunctionLibrary|GlTFLoadAssetfromUrl "https://github.com/cafragachan/gltf_data/blob/main/chair.glb?raw=true" (delegate Custom|LoadAsset))
  (bind _output_get (Variables|Default|SetPSComp (Actor|GetComponentbyClass "/Script/PixelStreaming.PixelStreamerInputComponent")))
  (EventDispatchers|BindEventtoOnInputEvent _output_get (delegate Custom|CustomEvent_1)))

(event Input|KeyboardEvents|SpaceBar
  (params (Key :type Key%20Structure :default "None")))

(event Input|MouseEvents|LeftMouseButton
  (params (Key :type Key%20Structure :default "None"))
  (:Pressed
    (Development|PrintString (Utilities|GetDisplayName (.hitactor (.HitResult (Game|Player|GetHitResultUnderCursorbyChannel "TraceTypeQuery1" false)))) true true "(R=0.370373,G=0.000000,B=1.000000,A=1.000000)" 2e+01)))

(event Input|TouchEvents|InputTouch
  (params (Location :type Vector) (FingerIndex :type ETouchIndex%20Enum))
  (:Pressed
    (Variables|Default|SetFinger%20Index FingerIndex)))

(fn ConstructionScript)