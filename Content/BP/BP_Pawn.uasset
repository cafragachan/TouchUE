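; Camera pawn that rotates the view by adding yaw and inverted pitch controller input from mouse axes every Tick.
; Touch-drag orbit, based on finger position deltas, and the call to pinch zoom are present but disconnected, so neither runs.
; ZoomInput turns changes in pinch value into a ratio for ZoomCamera, which moves the pawn along the controller's forward vector.
; Left-mouse and zoom prints are debug output.
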(event EventBeginPlay)

(event Collision|EventActorBeginOverlap
  (params (OtherActor :type Actor%20Object%20Reference)))

(event EventTick
  (params (DeltaSeconds :type Float%20%28single-precision%29))
  (bind _returnvalue (Game|Player|GetPlayerPawn 0))
  ;[1 1 1] Orbit Camera Mouse
  (Pawn|Input|AddControllerYawInput _returnvalue (Class|Actor|GetInputAxisKeyValue))
  (Pawn|Input|AddControllerPitchInput _returnvalue (* (Class|Actor|GetInputAxisKeyValue) -1.0)))

(event Input|AxisEvents|InputAxisPinchZoom
  (params (AxisValue :type Float%20%28single-precision%29)))

(event Input|KeyboardEvents|GesturePinch
  (params (Key :type Key%20Structure :default "None"))
  (:Pressed
    (Variables|Default|SetbScreenTouched false)))

(event Input|MouseEvents|LeftMouseButton
  (params (Key :type Key%20Structure :default "None"))
  (:Pressed
    (Development|PrintString "mmmmmmmmmmmmmmmmmmmmmmmmmmmmmmmmmmmmm" true true "(R=1.000000,G=0.679530,B=0.000000,A=1.000000)"))
  (:Released
    (Development|PrintString "hhhhhhhhhhhhhhhhhhhhhhhhhhhhhhhhhhhhhhhhhhhhhh" true true "(R=0.000000,G=1.000000,B=0.164242,A=1.000000)")))

(event Input|TouchEvents|InputTouch
  (params (Location :type Vector) (FingerIndex :type ETouchIndex%20Enum))
  ;[1 1 1] Orbit Camera touch
  (:Moved
    (Variables|Default|SetFinger%20Index FingerIndex)))

(event Input|TouchEvents|InputTouch
  (params (Location :type Vector) (FingerIndex :type ETouchIndex%20Enum))
  ;[1 1 1] Orbit Camera touch
  (:Pressed
    (Variables|Default|SetFinger%20Index FingerIndex)))

(fn ConstructionScript)

(fn ZoomCamera
  (params (scale :type Float%20%28single-precision%29))
  (Transformation|AddActorWorldOffset (* (Transformation|GetActorForwardVector (Pawn|GetController)) (* scale 5e+02))))

(fn ZoomInput
  (params (zoomScale :type Float%20%28single-precision%29))
  (if (not (== zoomScale (Variables|Default|GetPinchValue)))
    (Math|Float|CompareFloat zoomScale (Variables|Default|GetPinchValue)
      (:>
        (Development|PrintString (Utilities|String|ToString(Float) (- 1.0 (/ (Variables|Default|GetPinchValue) zoomScale))))
        (CallFunction|ZoomCamera (- 1.0 (/ (Variables|Default|GetPinchValue) zoomScale))))
      (:<
        (Development|PrintString (Utilities|String|ToString(Float) (- (/ zoomScale (Variables|Default|GetPinchValue)) 1.0)) true true "(R=1.000000,G=0.000000,B=0.000000,A=1.000000)")
        (CallFunction|ZoomCamera (- (/ zoomScale (Variables|Default|GetPinchValue)) 1.0))))
    (Variables|Default|SetPinchValue zoomScale)))